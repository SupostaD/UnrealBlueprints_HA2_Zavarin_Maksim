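; BP_BulletBase is a projectile that damages guards on impact.
; On spawn it launches its Sphere component forward with a velocity-change physics impulse and sets a short lifespan.
; When the Sphere hits a BP_GuardBase that implements BPI_Damageable, it calls ApplyDamage on that guard with its Damage value.
; Any hit destroys the bullet, whether or not damage is applied.
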(event `self.ReceiveBeginPlay`
  (`PrimitiveComponent.AddImpulse` (`self.Sphere`) (* (`self.GetActorForwardVector`) (`self.ImpulseStrength`)) "None" true)
  (`self.SetLifeSpan` 3.0))

(event `self.ReceiveActorBeginOverlap`
  (params (OtherActor :type "Actor Object Reference")))

(event `self.ReceiveTick`
  (params (DeltaSeconds :type "Float (single-precision)")))

(event `self.Sphere.OnComponentHit`
  (params (HitComponent :type "PrimitiveComponent Object Reference") (OtherActor :type "Actor Object Reference") (OtherComp :type "PrimitiveComponent Object Reference") (NormalImpulse :type "Vector Structure") (Hit :type "HitResult Structure (by ref)"))
  (bind _asbp_guard_base (cast `/Game/02_Zavarin_Maksim/Blueprints/Guard/BP_GuardBase` OtherActor)
    (:`then`
      (if (`KismetSystemLibrary.DoesClassImplementInterface` (`GameplayStatics.GetObjectClass` _asbp_guard_base) "/Game/02_Zavarin_Maksim/Blueprints/Interfaces/BPI_Damageable.BPI_Damageable_C")
        (`/Game/02_Zavarin_Maksim/Blueprints/Guard/BP_GuardBase.ApplyDamage` _asbp_guard_base (`self.Damage`))))
    (:`CastFailed`
      _))
  (`self.K2_DestroyActor`))

(fn `UserConstructionScript`)