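; BP_Magazine_Spawner scatters weapon magazine pickups inside a box volume when play begins.
; For each of SpawnCount iterations it picks a random point within SpawnBounds, projects it onto the navigation mesh, and spawns a random class from MagazineClasses there, adjusting for collisions.
; Each spawned magazine then randomizes its bullet count.
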(event `self.ReceiveBeginPlay`
  (bind _spawnbounds (`self.SpawnBounds`))
  (for _ (range (`self.SpawnCount`))
    (bind _returnvalue (`KismetMathLibrary.RandomPointInBoundingBox` (`SceneComponent.K2_GetComponentLocation` _spawnbounds) (`BoxComponent.GetScaledBoxExtent` _spawnbounds)))
    (bind _outitem (`KismetArrayLibrary.Array_Random` (`self.MagazineClasses`)))
    (bind _returnvalue_2 (`|SpawnActorFromClass` _outitem (`KismetMathLibrary.Conv_VectorToTransform` (`NavigationSystemV1.K2_ProjectPointToNavigation` _returnvalue null null (200.0 200.0 500.0))) "AdjustIfPossibleButAlwaysSpawn" "MultiplyWithRoot" null null))
    (`/Game/02_Zavarin_Maksim/Blueprints/Weapon/BP_MagazineBase.RandomizeAmountOfBullets` _returnvalue_2)))

(fn `UserConstructionScript`)