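; BP_MagazineBase is a base magazine actor with a bullet count and an ammo widget component.
; UpdateAmmoWidget pushes MagazineBullets into its WBP_MagazineAmmo widget.
; Its overlap handler finds BP_FirstPersonCharacter, but the AmmoPickup and destroy step sits behind a constant-false branch, so it never runs.
; RandomizeAmountOfBullets is an empty stub.
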(event `self.ReceiveBeginPlay`)

(event `self.ReceiveActorBeginOverlap`
  (params (OtherActor :type "Actor Object Reference"))
  (bind _returnvalue (`GameplayStatics.GetActorOfClass` "/Game/02_Zavarin_Maksim/BP_FirstPersonCharacter.BP_FirstPersonCharacter_C"))
  (if false
    (`/Game/02_Zavarin_Maksim/BP_FirstPersonCharacter.AmmoPickup` _returnvalue self)
    (`self.K2_DestroyActor`)))

(fn `RandomizeAmountOfBullets`)

(fn `UpdateAmmoWidget`
  (bind _aswbp_magazine_ammo (cast `/Game/02_Zavarin_Maksim/Blueprints/UI/WBP_MagazineAmmo` (`WidgetComponent.GetUserWidgetObject` (`self.AmmoWidget`))))
  (`/Game/02_Zavarin_Maksim/Blueprints/UI/WBP_MagazineAmmo.SetAmmoUI` _aswbp_magazine_ammo (`self.MagazineBullets`)))

(fn `UserConstructionScript`)