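; BP_Weapon2 is a pickup actor that gives the first-person character the second weapon.
; On overlap it finds BP_FirstPersonCharacter by class, sets its weapon-owned flag and ammo from BulletCount, equips the gun, then destroys itself.
; The overlapping actor is never checked, so any overlap triggers the pickup for that character.
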(event `self.ReceiveActorBeginOverlap`
  (params (OtherActor :type "Actor Object Reference"))
  (`parent.ReceiveActorBeginOverlap` OtherActor)
  (bind _returnvalue (`GameplayStatics.GetActorOfClass` "/Game/01_Zavarin_Maksim/BP_FirstPersonCharacter.BP_FirstPersonCharacter_C"))
  (set `/Game/01_Zavarin_Maksim/BP_FirstPersonCharacter.HasWeapon2` true _returnvalue)
  (set `/Game/01_Zavarin_Maksim/BP_FirstPersonCharacter.AmmoWeapon2` (`self.BulletCount`) _returnvalue)
  (`/Game/01_Zavarin_Maksim/BP_FirstPersonCharacter.EquipGun` _returnvalue "NewEnumerator1")
  (`self.K2_DestroyActor`))

(fn `UserConstructionScript`
  (`parent.UserConstructionScript`))