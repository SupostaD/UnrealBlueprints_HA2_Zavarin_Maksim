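; Base guard AI that patrols points, detects the player and gives chase, ending the game on capsule contact.
; Tick runs a Patrol/Track/Chase/Return state machine with per-state materials, using line-of-sight traces and DetectSphere overlap for detection.
; Timers decide Track-to-Chase escalation and chase give-up, after which the guard returns to the closest patrol point.
; ApplyDamage reduces health and destroys the guard at zero.
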(event `self.ReceiveBeginPlay`
  (bind _returnvalue (`GameplayStatics.GetActorOfClass` "/Game/01_Zavarin_Maksim/BP_FirstPersonCharacter.BP_FirstPersonCharacter_C"))
  (set `self.PlayerRef` _returnvalue)
  (set `self.GuardState` "NewEnumerator0")
  (set `self.PatrolIndex` 0)
  (set `self.Health` (`self.MaxHealth`)))

(event `self.ReceiveActorBeginOverlap`
  (params (OtherActor :type "Actor Object Reference")))

(event `self.ReceiveTick`
  (params (DeltaSeconds :type "Float (single-precision)"))
  (bind _playerref (`self.PlayerRef`))
  (bind _mesh (`self.Mesh`))
  (bind _outhit (`KismetSystemLibrary.LineTraceSingle` (`self.K2_GetActorLocation`) (`self.K2_GetActorLocation` _playerref) "TraceTypeQuery1"))
  (switch `/Game/01_Zavarin_Maksim/Blueprints/E_GuardState` (`self.GuardState`)
    (:`NewEnumerator0`
      (`PrimitiveComponent.SetMaterial` _mesh 0 "/Engine/EditorMaterials/GuardPatrolMat.GuardPatrolMat")
      (bind _returnvalue (== (`.HitActor` (`GameplayStatics.BreakHitResult` _outhit)) _playerref))
      (bind _returnvalue_2 (and _returnvalue (`self.isPlayerInArea`)))
      (if _returnvalue_2
        (`Controller.StopMovement` (`self.GetController`))
        (set `self.GuardState` "NewEnumerator1")
        (else
          (`self.GoToNextPatrolPoint`)
          (`self.CheckPatrolArrival`))))
    (:`NewEnumerator1`
      (`PrimitiveComponent.SetMaterial` _mesh 0 "/Engine/EditorMaterials/GuardTrackMat.GuardTrackMat")
      (if _returnvalue
        (`self.GuardRotation`)
        (bind _returnvalue_3 (`self.TrackTimer`))
        (if _returnvalue_3
          (set `self.TrackTime` 0.0)
          (if _returnvalue_2
            (`self.OnTrackSucceeded`)
            (else
              (`self.OnTrackFailed` :!label _label))))
        (else
          (goto _label))))
    (:`NewEnumerator2`
      (`PrimitiveComponent.SetMaterial` _mesh 0 "/Engine/EditorMaterials/GuardChaseMat.GuardChaseMat")
      (`self.GuardRotation`)
      (`|AIMoveTo` self (0.0 0.0 0.0) _playerref
        (:`then`
          (bind _returnvalue_4 (`self.ChaseGiveUpTimer`))
          (if _returnvalue_4
            (set `self.GiveUpTime` 0.0)
            (`self.OnChaseFailed`)))))
    (:`NewEnumerator3`
      (`PrimitiveComponent.SetMaterial` _mesh 0 "/Engine/EditorMaterials/GuardPatrolMat.GuardPatrolMat")
      (bind _closestpoint (`self.FindClosestPatrolPoint`))
      (`|AIMoveTo` self (0.0 0.0 0.0) _closestpoint
        (:`OnSuccess`
          (set `self.GuardState` "NewEnumerator0"))))))

(event `self.DetectSphere.OnComponentBeginOverlap`
  (params (OverlappedComponent :type "PrimitiveComponent Object Reference") (OtherActor :type "Actor Object Reference") (OtherComp :type "PrimitiveComponent Object Reference") (OtherBodyIndex :type Integer) (bFromSweep :type Boolean) (SweepResult :type "HitResult Structure (by ref)"))
  (cast `/Game/01_Zavarin_Maksim/BP_FirstPersonCharacter` OtherActor)
  (set `self.isPlayerInArea` true))

(event `self.DetectSphere.OnComponentEndOverlap`
  (params (OverlappedComponent :type "PrimitiveComponent Object Reference") (OtherActor :type "Actor Object Reference") (OtherComp :type "PrimitiveComponent Object Reference") (OtherBodyIndex :type Integer))
  (cast `/Game/01_Zavarin_Maksim/BP_FirstPersonCharacter` OtherActor)
  (set `self.isPlayerInArea` false))

(event `OnTrackSucceeded`
  (set `self.GuardState` "NewEnumerator2"))

(event `OnTrackFailed`
  (set `self.TrackTime` 0.0)
  (set `self.GuardState` "NewEnumerator0"))

(event `OnChaseFailed`
  (set `self.GuardState` "NewEnumerator3"))

(event `self.CapsuleComponent.OnComponentBeginOverlap`
  (params (OverlappedComponent :type "PrimitiveComponent Object Reference") (OtherActor :type "Actor Object Reference") (OtherComp :type "PrimitiveComponent Object Reference") (OtherBodyIndex :type Integer) (bFromSweep :type Boolean) (SweepResult :type "HitResult Structure (by ref)"))
  (cast `/Game/01_Zavarin_Maksim/BP_FirstPersonCharacter` OtherActor)
  (`GameplayStatics.SetGamePaused` true)
  (`KismetSystemLibrary.PrintString` "Game Over!" true true (struct :`R` 1.0 :`A` 1.0) 30.0)
  (`KismetSystemLibrary.Delay` 30.0)
  (`GameplayStatics.SetGamePaused` false)
  (`GameplayStatics.OpenLevel` "01_Zavarin_Maksim"))

(event `/Game/01_Zavarin_Maksim/Blueprints/BPI_Damageable.ApplyDamage`
  (params (Damage :type Integer))
  (bind _output_get (set `self.Health` (- (`self.Health`) Damage)))
  (if (<= _output_get 0)
    (set `self.Health` 0)
    (`|ExecutionSequence`
      (:`then_0`
        (`KismetSystemLibrary.PrintString` (`KismetStringLibrary.Conv_IntToString` _output_get) true true (struct :`G` 1.0 :`A` 1.0) 5.0 :!label _label_2))
      (:`then_1`
        (`self.K2_DestroyActor`)))
    (else
      (goto _label_2))))

(fn `ChaseGiveUpTimer`
  (returns (ReturnValue :type Boolean))
  (bind _output_get (set `self.GiveUpTime` (+ (`self.GiveUpTime`) (`GameplayStatics.GetWorldDeltaSeconds`))))
  (return (>= _output_get (`self.GiveUpTimeLimit`))))

(fn `CheckPatrolArrival`
  (bind _patrolpoints (`self.PatrolPoints`))
  (bind _patrolindex (`self.PatrolIndex`))
  (bind _returnvalue (`KismetArrayLibrary.Array_Length` _patrolpoints))
  (switch `/Game/01_Zavarin_Maksim/Blueprints/E_GuardState` (`self.GuardState`)
    (:`NewEnumerator0`
      (if (> _returnvalue 0)
        (if (<= (`KismetMathLibrary.Vector_Distance` (`self.K2_GetActorLocation`) (`self.K2_GetActorLocation` (`|GetArrayItem` _patrolpoints _patrolindex))) (`self.PatrolAcceptanceRadius`))
          (set `self.PatrolIndex` (mod (+ _patrolindex 1) _returnvalue))
          (`self.GoToNextPatrolPoint`))))))

(fn `FindClosestPatrolPoint`
  (returns (ClosestPoint :type "/Game/01_Zavarin_Maksim/Blueprints/BP_PatrolPoint Object Reference"))
  (set `self.ClosestDistance` 999999999999.0)
  (for _array_element (`self.PatrolPoints`)
    (bind _returnvalue (`self.K2_GetActorLocation` _array_element))
    (bind _returnvalue_2 (`KismetMathLibrary.Vector_Distance` _returnvalue (`self.K2_GetActorLocation` self)))
    (if (< _returnvalue_2 (`self.ClosestDistance`))
      (set `self.ClosestDistance` _returnvalue_2)
      (bind _output_get (set `self.ClosestPoint` _array_element))))
  (return _output_get))

(fn `GoToNextPatrolPoint`
  (bind _patrolpoints (`self.PatrolPoints`))
  (if (> (`KismetArrayLibrary.Array_Length` _patrolpoints) 0)
    (`AIBlueprintHelperLibrary.SimpleMoveToActor` (`self.GetController`) (`|GetArrayItem` _patrolpoints (`self.PatrolIndex`)))))

(fn `GuardRotation`
  (bind _returnvalue (`KismetMathLibrary.FindLookAtRotation` (`self.K2_GetActorLocation`) (`self.K2_GetActorLocation` (`self.PlayerRef`))))
  (bind (_roll _pitch _yaw) (`KismetMathLibrary.BreakRotator` _returnvalue))
  (bind _returnvalue_2 (`KismetMathLibrary.MakeRotator` 0.0 0.0 _yaw))
  (`self.K2_SetActorRotation` _returnvalue_2)
  (return))

(fn `RestartLevel`
  (`GameplayStatics.SetGamePaused` false)
  (`GameplayStatics.OpenLevel` "01_Zavarin_Maksim"))

(fn `TrackTimer`
  (returns (ReturnValue :type Boolean))
  (bind _output_get (set `self.TrackTime` (+ (`self.TrackTime`) (`GameplayStatics.GetWorldDeltaSeconds`))))
  (return (>= _output_get (`self.TrackTimeLimit`))))

(fn `UserConstructionScript`)