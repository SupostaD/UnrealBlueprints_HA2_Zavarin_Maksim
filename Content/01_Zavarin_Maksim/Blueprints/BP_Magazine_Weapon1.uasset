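; BP_Magazine_Weapon1 is the ammo pickup for Weapon 1, a child Blueprint that specializes an inherited magazine class.
; It sets its bullet weapon type on BeginPlay and overrides RandomizeAmountOfBullets to roll its own random bullet count.
; On any overlap it finds the first-person character via GetActorOfClass, ignoring OtherActor, and, if that character has Weapon 1, passes itself to AmmoPickup and destroys itself.
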(event `self.ReceiveBeginPlay`
  (`parent.ReceiveBeginPlay`)
  (set `self.BulletWeaponType` "NewEnumerator0"))

(event `self.ReceiveActorBeginOverlap`
  (params (OtherActor :type "Actor Object Reference"))
  (`parent.ReceiveActorBeginOverlap` OtherActor)
  (bind _returnvalue (`GameplayStatics.GetActorOfClass` "/Game/01_Zavarin_Maksim/BP_FirstPersonCharacter.BP_FirstPersonCharacter_C"))
  (if (`/Game/01_Zavarin_Maksim/BP_FirstPersonCharacter.HasWeapon1` _returnvalue)
    (`/Game/01_Zavarin_Maksim/BP_FirstPersonCharacter.AmmoPickup` _returnvalue self)
    (`self.K2_DestroyActor`)))

(fn `RandomizeAmountOfBullets`
  (`parent.RandomizeAmountOfBullets`)
  (set `self.MagazineBullets` (`KismetMathLibrary.RandomIntegerInRange` 10 20)))

(fn `UserConstructionScript`
  (`parent.UserConstructionScript`))